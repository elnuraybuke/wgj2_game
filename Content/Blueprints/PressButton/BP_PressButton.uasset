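; BP_PressButton is a pressable button linked to the witch boiler.
; On BeginPlay it caches the first BP_Witch_Boiler found in the level.
; Its Press event prints the boiler's red, yellow, blue and green potion values as a debug string, then flashes Cube1 red for a second before returning it to black.
; The trailing branch after the flash leads nowhere, so pressing triggers no other logic.
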(event `self.ReceiveBeginPlay`
  (bind _outactors (`GameplayStatics.GetAllActorsOfClass` "/Game/Blueprints/Witch_Boiler/BP_Witch_Boiler.BP_Witch_Boiler_C"))
  (set `self.Witch_Boiler` (`|GetArrayItem` _outactors)))

(event `/Game/Blueprints/Interfaces/BPI_IsCanPress.Press`
  (bind _witch_boiler (`self.Witch_Boiler`))
  (`KismetSystemLibrary.PrintString` (`KismetTextLibrary.Conv_TextToString` (`|FormatText` "RedPotion: {RED} \nYellowPotion: {Yellow} \nBluePotion: {Blue} \nGreenPotion:{Green}" (`/Game/Blueprints/Witch_Boiler/BP_Witch_Boiler.RedPotion` _witch_boiler) (`/Game/Blueprints/Witch_Boiler/BP_Witch_Boiler.YellowPotion` _witch_boiler) (`/Game/Blueprints/Witch_Boiler/BP_Witch_Boiler.BluePotion` _witch_boiler) (`/Game/Blueprints/Witch_Boiler/BP_Witch_Boiler.GreenPotion` _witch_boiler))) true true (struct :`G` 0.66 :`B` 1.0 :`A` 1.0) 100.0 "Nonsae")
  (`PrimitiveComponent.SetMaterial` (`self.Cube1`) 0 "/Game/Materials/PotionMaterial/M_Red.M_Red")
  (`KismetSystemLibrary.Delay` 1.0)
  (`PrimitiveComponent.SetMaterial` (`self.Cube1`) 0 "/Game/Materials/PotionMaterial/M_Black.M_Black")
  (if true
    _))

(fn `UserConstructionScript`)