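; Witch boiler actor that collects colored potions dropped into its box trigger and keeps a count for each color.
; On overlap, a sequence of casts identifies a blue, red, green or yellow potion and increments the matching counter.
; The matched potion then clears its message and is destroyed, and the cached BP_Ally reference is flagged as no longer holding an item.
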(event `self.ReceiveBeginPlay`
  (bind _outactors (`GameplayStatics.GetAllActorsOfClass` "/Game/Blueprints/Potion/BP_Potion.BP_Potion_C"))
  (set `self.BP_Potion_Ref` (`|GetArrayItem` _outactors))
  (bind _outactors_2 (`GameplayStatics.GetAllActorsOfClass` "/Game/Blueprints/Character/BP_Ally.BP_Ally_C"))
  (set `self.BP_Ally_Ref` (`|GetArrayItem` _outactors_2)))

(event `self.Box.OnComponentBeginOverlap`
  (params (OverlappedComponent :type "PrimitiveComponent Object Reference") (OtherActor :type "Actor Object Reference") (OtherComp :type "PrimitiveComponent Object Reference") (OtherBodyIndex :type Integer) (bFromSweep :type Boolean) (SweepResult :type "HitResult Structure (by ref)"))
  (bind _asbp_potion (cast `/Game/Blueprints/Potion/BP_Potion` OtherActor))
  ; Potion_Check
  (`|ExecutionSequence`
    (:`then_0`
      (bind _asbp_blue_potion (cast `/Game/Blueprints/Potion/BP_BluePotion` _asbp_potion))
      (bind _output_get (set `self.BluePotion` (+ (`self.BluePotion`) 1)))
      (message `/Game/Blueprints/Interfaces/BPI_CanTake.TakeOff` _asbp_blue_potion)
      (`self.K2_DestroyActor` _asbp_blue_potion)
      (set `/Game/Blueprints/Character/BP_Ally.HaveItemOnHands?` false (`self.BP_Ally_Ref`)))
    (:`then_1`
      (bind _asbp_red_potion (cast `/Game/Blueprints/Potion/BP_RedPotion` _asbp_potion))
      (bind _output_get_2 (set `self.RedPotion` (+ (`self.RedPotion`) 1)))
      (message `/Game/Blueprints/Interfaces/BPI_CanTake.TakeOff` _asbp_red_potion)
      (`self.K2_DestroyActor` _asbp_red_potion)
      (set `/Game/Blueprints/Character/BP_Ally.HaveItemOnHands?` false (`self.BP_Ally_Ref`)))
    (:`then_2`
      (bind _asbp_green_potion (cast `/Game/Blueprints/Potion/BP_GreenPotion` _asbp_potion))
      (bind _output_get_3 (set `self.GreenPotion` (+ (`self.GreenPotion`) 1)))
      (message `/Game/Blueprints/Interfaces/BPI_CanTake.TakeOff` _asbp_green_potion)
      (`self.K2_DestroyActor` _asbp_green_potion)
      (set `/Game/Blueprints/Character/BP_Ally.HaveItemOnHands?` false (`self.BP_Ally_Ref`)))
    (:`then_3`
      (bind _asbp_yellow_potion (cast `/Game/Blueprints/Potion/BP_YellowPotion` _asbp_potion))
      (bind _output_get_4 (set `self.YellowPotion` (+ (`self.YellowPotion`) 1)))
      (message `/Game/Blueprints/Interfaces/BPI_CanTake.TakeOff` _asbp_yellow_potion)
      (`self.K2_DestroyActor` _asbp_yellow_potion)
      (set `/Game/Blueprints/Character/BP_Ally.HaveItemOnHands?` false (`self.BP_Ally_Ref`)))))

(fn `UserConstructionScript`)