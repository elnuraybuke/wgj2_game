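; An NPC that walks to the BP_Location_1 actor on BeginPlay and brings up the missions widget.
; A timeline lerps its current location toward that actor during the walking animation.
; A delay chained to the timeline's update switches it to idle and adds W_Missions to the viewport.
; A separate MakeOrder event picks a random order from OrderData and prints its item types and counts.
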(event `self.ReceiveBeginPlay`
  (bind _outactors (`GameplayStatics.GetAllActorsOfClass` "/Game/Blueprints/LocationPoints/BP_Location_1.BP_Location_1_C"))
  (set `self.BP_Location_1` (`|GetArrayItem` _outactors))
  (`SkeletalMeshComponent.PlayAnimation` (`self.Mesh`) "/Game/Blueprints/Npcs/Npc_BossAndAnimaton/Animaton/Walking_Anim.Walking_Anim" true)
  (bind (_direction _movedataofboss) (`Timeline|Timeline`)
    (:`Update`
      (`self.K2_SetActorLocation` (`KismetMathLibrary.VLerp` (`self.K2_GetActorLocation`) (`self.K2_GetActorLocation` (`self.BP_Location_1`)) _movedataofboss))
      (`KismetSystemLibrary.Delay` 4.0)
      (`SkeletalMeshComponent.PlayAnimation` (`self.Mesh`) "/Game/Blueprints/Npcs/Npc_BossAndAnimaton/Animaton/Idle_Anim.Idle_Anim" false)
      (bind _returnvalue (`|CreateWidget` "/Game/Blueprints/Widgets/W_Missions.W_Missions_C"))
      (`UserWidget.AddToViewport` _returnvalue 0))))

(event `MakeOrder`
  (bind _orderdata_order_0 (break `/Game/S_OrderData` (`self.OrderData`)))
  (bind _output_get (set `self.CurrentOrder` (`KismetMathLibrary.RandomInteger` (`KismetArrayLibrary.Array_Length` _orderdata_order_0))))
  (bind _output_item (break `/Game/S_Order` (`|GetArrayItem` _orderdata_order_0 _output_get)))
  (`|MapForEach` _output_item
    (:`then`
      (`KismetSystemLibrary.PrintString` (`KismetTextLibrary.Conv_TextToString` (`|FormatText` "Item {itemType}, Count {count}" _ _))))))

(fn `UserConstructionScript`)