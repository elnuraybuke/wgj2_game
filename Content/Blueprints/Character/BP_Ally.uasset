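; BP_Ally is a player-controlled character that moves, looks, picks up items and presses interactable objects.
; BeginPlay registers an Enhanced Input mapping context, whose actions drive control-rotation-relative movement and controller look.
; The interact action either drops the held item or line-traces from the camera with debug drawing, then messages the hit actor through the BPI_CanTake or BPI_IsCanPress interface, tracking the held state.
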(event `self.ReceiveBeginPlay`
  (bind _asplayer_controller (cast `PlayerController` (`self.GetController`)))
  (`EnhancedInputSubsystemInterface.AddMappingContext` (pcsubsystem `EnhancedInputLocalPlayerSubsystem` _asplayer_controller) "/Game/InputS/IMP_BaseContext.IMP_BaseContext" 0 (struct)))

(event `EnhancedInput|/Game/InputS/Input_Actions/IA_Move`
  (params (ActionValue :type "Vector2D Structure") (ElapsedSeconds :type "Float (double-precision)") (TriggeredSeconds :type "Float (double-precision)") (InputAction :type "InputAction Object Reference" :default "/Game/InputS/Input_Actions/IA_Move.IA_Move"))
  (bind (_x _y) (`KismetMathLibrary.BreakVector2D` ActionValue))
  (:`Triggered`
    (`PawnMovementComponent.AddInputVector` (`self.CharacterMovement`) (* (`KismetMathLibrary.GetForwardVector` (`self.GetControlRotation`)) _x) false)
    (`PawnMovementComponent.AddInputVector` (`self.CharacterMovement`) (* (`KismetMathLibrary.GetRightVector` (`self.GetControlRotation`)) _y) false)))

(event `EnhancedInput|/Game/InputS/Input_Actions/IA_Look`
  (params (ActionValue :type "Vector2D Structure") (ElapsedSeconds :type "Float (double-precision)") (TriggeredSeconds :type "Float (double-precision)") (InputAction :type "InputAction Object Reference" :default "/Game/InputS/Input_Actions/IA_Look.IA_Look"))
  (bind (_x _y) (`KismetMathLibrary.BreakVector2D` ActionValue))
  (:`Triggered`
    (`self.AddControllerYawInput` _x)
    (`self.AddControllerPitchInput` _y)))

(event `EnhancedInput|/Game/InputS/Input_Actions/IA_GetSomething`
  (params (ActionValue :type Boolean) (ElapsedSeconds :type "Float (double-precision)") (TriggeredSeconds :type "Float (double-precision)") (InputAction :type "InputAction Object Reference" :default "/Game/InputS/Input_Actions/IA_GetSomething.IA_GetSomething"))
  (bind _camera (`self.Camera`))
  (bind _returnvalue (`SceneComponent.K2_GetComponentLocation` _camera))
  ; Take_Item
  (:`Started`
    (if (`self.HaveItemOnHands?`)
      (message `/Game/Blueprints/Interfaces/BPI_CanTake.TakeOff` (`self.FastRef`))
      (set `self.HaveItemOnHands?` false)
      (else
        (bind _outhit (`KismetSystemLibrary.LineTraceSingle` :`Start` _returnvalue :`End` (+ _returnvalue (* (`KismetMathLibrary.GetForwardVector` (`SceneComponent.K2_GetComponentRotation` _camera)) (`self.TakeItemDistance`))) :`TraceChannel` "TraceTypeQuery1" :`DrawDebugType` "ForDuration" :`DrawTime` 10.0))
        (bind (_bblockinghit _binitialoverlap _time _distance _location _impactpoint _normal _impactnormal _physmat _hitactor) (`GameplayStatics.BreakHitResult` _outhit))
        (set `self.FastRef` _hitactor)
        (if (`KismetSystemLibrary.DoesImplementInterface` _hitactor "/Game/Blueprints/Interfaces/BPI_CanTake.BPI_CanTake_C")
          (message `/Game/Blueprints/Interfaces/BPI_CanTake.TakeItems` _hitactor)
          (set `self.HaveItemOnHands?` true)
          (elif (`KismetSystemLibrary.DoesImplementInterface` _hitactor "/Game/Blueprints/Interfaces/BPI_IsCanPress.BPI_IsCanPress_C")
            (message `/Game/Blueprints/Interfaces/BPI_IsCanPress.Press` _hitactor)))))))

(fn `UserConstructionScript`)