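; BP_Potion is a physics-enabled potion actor that the BP_Ally character can carry and drop.
; On BeginPlay it caches the BP_Ally instance found with GetActorOfClass.
; TakeItems turns off physics and attaches to the ally's Scene component, keeping world location but relative rotation and scale.
; TakeOff re-enables physics and detaches the Potion component, keeping its world location.
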(event `self.ReceiveBeginPlay`
  (bind _returnvalue (`GameplayStatics.GetActorOfClass` "/Game/Blueprints/Character/BP_Ally.BP_Ally_C"))
  (set `self.BP_Ally_Ref` _returnvalue))

(event `/Game/Blueprints/Interfaces/BPI_CanTake.TakeItems`
  ; TakeItem
  (`PrimitiveComponent.SetSimulatePhysics` (`self.Potion`) false)
  (`self.K2_AttachToComponent` (`/Game/Blueprints/Character/BP_Ally.Scene` (`self.BP_Ally_Ref`)) "None" "KeepWorld" "KeepRelative" "KeepRelative"))

(event `/Game/Blueprints/Interfaces/BPI_CanTake.TakeOff`
  (`PrimitiveComponent.SetSimulatePhysics` (`self.Potion`) true)
  (`SceneComponent.K2_DetachFromComponent` (`self.Potion`) "KeepWorld" "KeepRelative" "KeepRelative" true))

(fn `UserConstructionScript`)